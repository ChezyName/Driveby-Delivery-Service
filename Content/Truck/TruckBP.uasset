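; Drivable truck pawn that a ThirdPersonCharacter can enter and exit, with a trigger that toggles pizza pickup on that character.
; Input stores throttle, steering and a toggled brake state, which Tick applies as per-wheel drive, steer and brake torques on VehicleMovement.
; Tick also drives skid effects, engine and screech audio.
; An overlap trigger offers entry; OnPossesed and the Enter action swap controller possession between character and truck.
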(event `InputAction|Honk`
  (params (Key :type "Key Structure"))
  (bind _honk (`self.Honk`))
  (:`Pressed`
    (`AudioComponent.Play` _honk 0.0))
  (:`Released`
    (`AudioComponent.Stop` _honk)))

(event `InputAction|Enter`
  (params (Key :type "Key Structure"))
  (bind _returnvalue (`self.GetController`))
  (bind _charonpossesed (`self.CharOnPossesed`))
  (:`Pressed`
    (if (`self.isPossesed`)
      (`AudioComponent.Stop` (`self.Honk`))
      (`Controller.Possess` _returnvalue _charonpossesed)
      (`/Game/ThirdPersonBP/Blueprints/ThirdPersonCharacter.RePossesChar` _charonpossesed)
      (set `self.CharOnPossesed` null)
      (set `self.isPossesed` false)
      (`Controller.UnPossess` _returnvalue))))

(event `self.ReceiveTick`
  (params (DeltaSeconds :type "Float (single-precision)"))
  (bind _tirescreach (`self.TireScreach`))
  (bind _braking (`self.Braking`))
  (`/Engine/EditorBlueprintResources/ActorMacros.Switch Has Authority`
    (:`Authority`
      _)
    (:`Remote`
      _))
  (`self.UpdateWheels` (* (`self.DriveSpeed`) 45000.0) (* (`self.SteerAngle`) 30.0))
  (`self.UpdateBrake`)
  (`self.CharUpdate`)
  (`ActorComponent.SetActive` (`self.L_Skid`) _braking false)
  (`ActorComponent.SetActive` (`self.R_Skid`) _braking false)
  (`ActorComponent.SetActive` (`self.L_SkidF`) _braking false)
  (`ActorComponent.SetActive` (`self.R_SkidF`) _braking false)
  (if (and (> (`WheeledVehicleMovementComponent.GetEngineRotationSpeed` (`self.VehicleMovement`)) 0.0) (`self.Braking`))
    (if (not (`AudioComponent.IsPlaying` _tirescreach))
      (`AudioComponent.Play` _tirescreach 0.0))
    (else
      (`AudioComponent.Stop` _tirescreach))))

(event `InputAction|Handbrake`
  (params (Key :type "Key Structure"))
  (bind _returnvalue (not (`self.Braking`)))
  (:`Pressed`
    (`WheeledVehicleMovementComponent.SetHandbrakeInput` (`self.VehicleMovement`) _returnvalue)
    (`self.ServerBraking` _returnvalue)))

(event `ServerBraking`
  (params (Brake :type Boolean))
  (set `self.Braking` Brake))

(event `OnBrake`
  (params (Broke :type Boolean))
  (if Broke
    (`AudioComponent.Play` (`self.BrakeActive`) 0.0)
    (else
      (`AudioComponent.Play` (`self.BrakeUnActive`) 0.0))))

(event `InputAxis|MoveRight` :overrideparent false
  (params (AxisValue :type "Float (single-precision)"))
  (`self.setSteerSpeed` AxisValue))

(event `setDriveSpeed`
  (params (Speed :type "Float (double-precision)"))
  (set `self.DriveSpeed` Speed))

(event `InputAxis|MoveForward` :overrideparent false
  (params (AxisValue :type "Float (single-precision)"))
  (`self.setDriveSpeed` AxisValue))

(event `setSteerSpeed`
  (params (Steer :type "Float (double-precision)"))
  (set `self.SteerAngle` Steer))

(event `InputAxis|Turn` :overrideparent false
  (params (AxisValue :type "Float (single-precision)"))
  (`self.AddControllerYawInput` AxisValue))

(event `InputAxis|LookUp` :overrideparent false
  (params (AxisValue :type "Float (single-precision)"))
  (`self.AddControllerPitchInput` AxisValue))

(event `self.EnterVehicle.OnComponentBeginOverlap`
  (params (OverlappedComponent :type "PrimitiveComponent Object Reference") (OtherActor :type "Actor Object Reference") (OtherComp :type "PrimitiveComponent Object Reference") (OtherBodyIndex :type Integer) (bFromSweep :type Boolean) (SweepResult :type "HitResult Structure (by ref)"))
  (`/Engine/EditorBlueprintResources/StandardMacros.IsValid` (`self.CharOnPossesed`)
    (:`Is Not Valid`
      (bind _asthird_person_character (cast `/Game/ThirdPersonBP/Blueprints/ThirdPersonCharacter` OtherActor))
      (set `self.Character` _asthird_person_character))))

(event `self.EnterVehicle.OnComponentEndOverlap`
  (params (OverlappedComponent :type "PrimitiveComponent Object Reference") (OtherActor :type "Actor Object Reference") (OtherComp :type "PrimitiveComponent Object Reference") (OtherBodyIndex :type Integer))
  (bind _asthird_person_character (cast `/Game/ThirdPersonBP/Blueprints/ThirdPersonCharacter` OtherActor))
  (set `self.Character` null)
  (`/Game/ThirdPersonBP/Blueprints/ThirdPersonCharacter.EnterVehicleDisplay` _asthird_person_character null))

(event `self.PizzaPickup.OnComponentBeginOverlap`
  (params (OverlappedComponent :type "PrimitiveComponent Object Reference") (OtherActor :type "Actor Object Reference") (OtherComp :type "PrimitiveComponent Object Reference") (OtherBodyIndex :type Integer) (bFromSweep :type Boolean) (SweepResult :type "HitResult Structure (by ref)"))
  (bind _asthird_person_character (cast `/Game/ThirdPersonBP/Blueprints/ThirdPersonCharacter` OtherActor))
  (`/Game/ThirdPersonBP/Blueprints/ThirdPersonCharacter.PizzaEnable` _asthird_person_character true))

(event `self.PizzaPickup.OnComponentEndOverlap`
  (params (OverlappedComponent :type "PrimitiveComponent Object Reference") (OtherActor :type "Actor Object Reference") (OtherComp :type "PrimitiveComponent Object Reference") (OtherBodyIndex :type Integer))
  (bind _asthird_person_character (cast `/Game/ThirdPersonBP/Blueprints/ThirdPersonCharacter` OtherActor))
  (`/Game/ThirdPersonBP/Blueprints/ThirdPersonCharacter.PizzaEnable` _asthird_person_character false))

(fn `CharUpdate`
  (bind _character (`self.Character`))
  (`/Engine/EditorBlueprintResources/StandardMacros.IsValid` _character
    (:`Is Valid`
      (`/Game/ThirdPersonBP/Blueprints/ThirdPersonCharacter.EnterVehicleDisplay` _character self))))

(fn `onPossesed`
  (params (Char :type "/Game/ThirdPersonBP/Blueprints/ThirdPersonCharacter Object Reference"))
  (`/Engine/EditorBlueprintResources/StandardMacros.IsValid` Char
    (:`Is Valid`
      (`Controller.Possess` (`self.GetController` Char) self)
      (set `self.isPossesed` true)
      (set `self.CharOnPossesed` Char)
      (`AudioComponent.Play` (`self.Enter`) 0.0))))

(fn `UpdateBrake`
  (bind _braking (`self.Braking`))
  (bind _vehiclemovement (`self.VehicleMovement`))
  (`KismetSystemLibrary.PrintString` (`KismetStringLibrary.Conv_BoolToString` _braking))
  (if _braking
    (`SimpleWheeledVehicleMovementComponent.SetBrakeTorque` _vehiclemovement 150000.0 4)
    (`SimpleWheeledVehicleMovementComponent.SetBrakeTorque` _vehiclemovement 150000.0 5)
    (`SimpleWheeledVehicleMovementComponent.SetBrakeTorque` _vehiclemovement 150000.0 2)
    (`SimpleWheeledVehicleMovementComponent.SetBrakeTorque` _vehiclemovement 150000.0 3)
    (else
      (`SimpleWheeledVehicleMovementComponent.SetBrakeTorque` _vehiclemovement 0.0 4)
      (`SimpleWheeledVehicleMovementComponent.SetBrakeTorque` _vehiclemovement 0.0 5)
      (`SimpleWheeledVehicleMovementComponent.SetBrakeTorque` _vehiclemovement 0.0 2)
      (`SimpleWheeledVehicleMovementComponent.SetBrakeTorque` _vehiclemovement 0.0 3))))

(fn `UpdateWheels`
  (params (DriveSpeed :type "Float (double-precision)") (Steering :type "Float (double-precision)"))
  (bind _enginedrive (`self.EngineDrive`))
  (bind _vehiclemovement (`self.VehicleMovement`))
  (bind _returnvalue (`KismetMathLibrary.SelectFloat` 0.0 DriveSpeed (`self.Braking`)))
  (`KismetSystemLibrary.PrintString` (`KismetStringLibrary.Concat_StrStr` (`KismetStringLibrary.Conv_DoubleToString` DriveSpeed) " @ " (`KismetStringLibrary.Conv_DoubleToString` Steering)))
  (`SimpleWheeledVehicleMovementComponent.SetDriveTorque` _vehiclemovement _returnvalue 2)
  (`SimpleWheeledVehicleMovementComponent.SetDriveTorque` _vehiclemovement _returnvalue 3)
  (`SimpleWheeledVehicleMovementComponent.SetDriveTorque` _vehiclemovement _returnvalue 4)
  (`SimpleWheeledVehicleMovementComponent.SetDriveTorque` _vehiclemovement _returnvalue 5)
  (`SimpleWheeledVehicleMovementComponent.SetSteerAngle` _vehiclemovement Steering 0)
  (`SimpleWheeledVehicleMovementComponent.SetSteerAngle` _vehiclemovement Steering 1)
  (if (>= (`KismetMathLibrary.Abs` (`WheeledVehicleMovementComponent.GetForwardSpeed` _vehiclemovement)) 1.0)
    (if (not (`AudioComponent.IsPlaying` _enginedrive))
      (`AudioComponent.Play` _enginedrive 0.0))
    (else
      (`AudioComponent.Stop` _enginedrive))))

(fn `UserConstructionScript`)